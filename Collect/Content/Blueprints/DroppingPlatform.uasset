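; Platform that sinks while the player character stands in its descent trigger and returns to its starting position once they leave.
; Trigger overlap events swap two looping timers, each using the current frame delta as its interval, instead of using Tick.
; The descent lowers the cube at FallingSpeed without a limit.
; The return interpolates at the same speed with sweep, stopping its timer near the origin saved at BeginPlay.
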(event OnComponentBeginOverlap(TriggerBoxDescent)
  (params (OverlappedComponent :type Primitive%20Component%20Object%20Reference) (OtherActor :type Actor%20Object%20Reference) (OtherComp :type Primitive%20Component%20Object%20Reference) (OtherBodyIndex :type Integer) (bFromSweep :type Boolean) (SweepResult :type Hit%20Result%20Structure%20%28by%20ref%29))
  (Utilities|Casting|CastToBP_ThirdPersonCharacter OtherActor)
  (Utilities|Time|SetTimerbyEvent (delegate Custom|MovePlatformDown) (Utilities|Time|GetWorldDeltaSeconds) true)
  (Utilities|Time|ClearTimerbyFunctionName 0 "MovePlatformUp"))

(event OnComponentEndOverlap(TriggerBoxDescent)
  (params (OverlappedComponent :type Primitive%20Component%20Object%20Reference) (OtherActor :type Actor%20Object%20Reference) (OtherComp :type Primitive%20Component%20Object%20Reference) (OtherBodyIndex :type Integer))
  (Utilities|Casting|CastToBP_ThirdPersonCharacter OtherActor)
  (Utilities|Time|ClearTimerbyFunctionName 0 "MovePlatformDown")
  (Utilities|Time|SetTimerbyEvent (delegate Custom|MovePlatformUp) (Utilities|Time|GetWorldDeltaSeconds) true))

(event Custom|MovePlatformDown
  (Transformation|AddRelativeLocation (Variables|Default|GetCube) (Math|Vector|MakeVector 0.0 0.0 (* (* (Utilities|Time|GetWorldDeltaSeconds) (Variables|Default|GetFalling%20Speed)) -1.0)) false false))

(event Custom|MovePlatformUp
  (Transformation|SetRelativeLocation (Variables|Default|GetCube) (Math|Interpolation|VInterptoConstant (Variables|/Script/Engine.SceneComponent|GetRelativeLocation (Variables|Default|GetCube)) (Variables|Components|GetOriginLocation) (Utilities|Time|GetWorldDeltaSeconds) (Variables|Default|GetFalling%20Speed)) true false)
  (if (Math|Float|NearlyEqual(Float) (Math|Vector|Distance(Vector) (Variables|/Script/Engine.SceneComponent|GetRelativeLocation (Variables|Default|GetCube)) (Variables|Components|GetOriginLocation)) 0.0 1.0)
    (Utilities|Time|ClearTimerbyFunctionName 0 "MovePlatformUp")))

(event EventBeginPlay
  (Variables|Components|SetOriginLocation (Variables|/Script/Engine.SceneComponent|GetRelativeLocation (Variables|Default|GetCube))))

(fn ConstructionScript)